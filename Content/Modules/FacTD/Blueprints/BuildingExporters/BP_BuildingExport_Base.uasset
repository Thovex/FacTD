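; Base building exporter for FacTD that gives each exported building entity a HISM mesh component built from its mesh and materials, with Visibility collision.
; The construction script finds its own class in the player controller's default building-constructor map to read the building size.
; It then adds a static mesh component at the center location, scaled in X and Y to that size, with the same mesh and materials.
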(event EventExportImplementation
  (params (CreatedEntity :type Integer))
  (Class|HismMeshComponentBlueprintLibrary|EmplaceHismMeshComponent CreatedEntity (Utilities|Struct|MakeHismMeshComponent (Variables|Default|GetMesh) (Variables|Default|GetMaterials) "ECC_Visibility")))

(fn ConstructionScript
  (bind _buildingconstructorblueprint (Utilities|GetClassDefaults "/Game/Modules/FacTD/Blueprints/BP_FacTD_PlayerController.BP_FacTD_PlayerController_C"))
  (bind _keys (Utilities|Map|Keys _buildingconstructorblueprint))
  (bind _array_element (Utilities|Array|ForEachLoopwithBreak _keys :!label _label)
    (:LoopBody
      (if (== (.buildingconstructor (.Value (Utilities|Map|Find _buildingconstructorblueprint _array_element))) (Utilities|GetClass self))
        (Variables|Default|SetBuildingSize (.buildingsize (.Value (Utilities|Map|Find _buildingconstructorblueprint _array_element))))
        (goto _label Break)))
    (:Completed
      (bind _returnvalue (AddComponent|AddStaticMeshComponent false (Math|Transform|MakeTransform (Variables|Default|GetCenterLocation) "0, 0, 0" (Math|Vector|MakeVector (Math|Conversions|ToFloat(Integer) (.x (Variables|Default|GetBuildingSize))) (Math|Conversions|ToFloat(Integer) (.y (Variables|Default|GetBuildingSize))) 1.0))))
      (Components|StaticMesh|SetStaticMesh _returnvalue (Variables|Default|GetMesh))
      (for (_array_element_2 _array_index) (Variables|Default|GetMaterials)
        (Rendering|Material|SetMaterial _returnvalue _array_index _array_element_2)))))