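; Player controller for the FacTD module that handles grid-based placement, removal and rotation of buildings.
; Each tick it draws a debug-shape preview of the selected building's footprint at the current grid position, with lines showing its facing.
; Q and E cycle that facing with wraparound, while left click, right click and R call TryConstruct, TryDestroy and TryRotate, none of which are defined in this Blueprint.
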(event EventTick
  (params (DeltaSeconds :type Float%20%28single-precision%29))
  (bind _returnvalue (Utilities|Time|GetWorldDeltaSeconds))
  (bind _currentgridposition (Variables|Default|GetCurrentGridPosition))
  (bind _selectedbuilding (Variables|Default|GetSelectedBuilding))
  (bind _buildingconstructorblueprint (Variables|Default|GetBuildingConstructorBlueprint))
  (bind _value (Utilities|Map|Find _buildingconstructorblueprint _selectedbuilding))
  (bind _returnvalue_2 (* _returnvalue 2.0))
  (|CallParentFunction DeltaSeconds)
  (for _index (range 0 (- (.x (.buildingsize _value)) 1))
    (for _index_2 (range 0 (- (.y (.buildingsize _value)) 1))
      (Rendering|Debug|DrawDebugBox (Math|Vector|MakeVector (* (Math|Conversions|ToFloat(Integer) (+ (.x _currentgridposition) _index)) 1e+02) (* (Math|Conversions|ToFloat(Integer) (+ (.y _currentgridposition) _index_2)) 1e+02) 0.0) "50.000000,50.000000,50.000000" "(R=0.112931,G=1.000000,B=0.049625,A=1.000000)" "0, 0, 0" _returnvalue_2 3.0)
      (Rendering|Debug|DrawDebugLine (+ (Math|Vector|MakeVector (* (Math|Conversions|ToFloat(Integer) (+ (.x _currentgridposition) _index)) 1e+02) (* (Math|Conversions|ToFloat(Integer) (+ (.y _currentgridposition) _index_2)) 1e+02) 0.0) "0.000000,0.000000,100.000000") (+ (+ (Math|Vector|MakeVector (* (Math|Conversions|ToFloat(Integer) (+ (.x _currentgridposition) _index)) 1e+02) (* (Math|Conversions|ToFloat(Integer) (+ (.y _currentgridposition) _index_2)) 1e+02) 0.0) "0.000000,0.000000,100.000000") (* (Class|FacTDBuildingUtil|ConvertBuildingDirection (Variables|Default|GetDirection)) 1e+02)) "(R=0.786458,G=0.000000,B=0.283063,A=1.000000)" _returnvalue_2 5.0))))

(event Input|MouseEvents|DebugKeyRightMouseButton
  (params (Key :type Key%20Structure :default "None") (ActionValue :type Input%20Action%20Value%20Structure))
  (:Pressed
    (Class|FacTDPlayerController|TryDestroy (Variables|Default|GetCurrentGridPosition))))

(event Input|KeyboardEvents|Q
  (params (Key :type Key%20Structure :default "None"))
  (:Pressed
    (if (< (- (Math|Conversions|ToInteger(Byte) (Variables|Default|GetDirection)) 1) 0)
      (Variables|Default|SetDirection "EFacTD_BuildingDirection_Left")
      (else
        (Variables|Default|SetDirection (Utilities|Enum|ByteToEnumEFacTD_BuildingDirection (Math|Conversions|ToByte(Integer) (- (Math|Conversions|ToInteger(Byte) (Variables|Default|GetDirection)) 1))))))))

(event Input|MouseEvents|LeftMouseButton
  (params (Key :type Key%20Structure :default "None"))
  (:Pressed
    (Class|FacTDPlayerController|TryConstruct (Variables|Default|GetSelectedBuilding) (Variables|Default|GetCurrentGridPosition) (Variables|Default|GetDirection))))

(event Input|KeyboardEvents|E
  (params (Key :type Key%20Structure :default "None"))
  (:Pressed
    (if (> (+ (Math|Conversions|ToInteger(Byte) (Variables|Default|GetDirection)) 1) 3)
      (Variables|Default|SetDirection "EFacTD_BuildingDirection_Up")
      (else
        (Variables|Default|SetDirection (Utilities|Enum|ByteToEnumEFacTD_BuildingDirection (Math|Conversions|ToByte(Integer) (+ (Math|Conversions|ToInteger(Byte) (Variables|Default|GetDirection)) 1))))))))

(event Input|KeyboardEvents|R
  (params (Key :type Key%20Structure :default "None"))
  (:Pressed
    (Class|FacTDPlayerController|TryRotate (Variables|Default|GetCurrentGridPosition))))

(fn ConstructionScript)